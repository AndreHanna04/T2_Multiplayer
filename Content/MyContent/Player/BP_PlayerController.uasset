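; Player controller that routes Enhanced Input to the possessed BP_Character and owns the local player's HUD, scoreboard and reload widgets.
; On possession, the local controller adds input contexts and creates the widgets once, hiding the scoreboard and reload bar.
; Helper functions swap attack and reload mapping contexts, drive the reload bar and update HUD ammo.
; Special reload input grants ammo if the character can critically reload, otherwise triggers a lockout.
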(event Input|EnhancedActionEvents|EnhancedInputActionIA_Move
  (params (ActionValue :type Vector :default "0, 0, 0") (ElapsedSeconds :type Float%20%28double-precision%29) (TriggeredSeconds :type Float%20%28double-precision%29) (InputAction :type Input%20Action%20Object%20Reference :default "/Game/MyContent/Player/Inputs/IA_Move.IA_Move"))
  (Class|MGCharacter|PureMoveCharacter (Variables|Default|GetCharRef) ActionValue))

(event Input|EnhancedActionEvents|EnhancedInputActionIA_TurnCamera
  (params (ActionValue :type Vector%202D%20Structure) (ElapsedSeconds :type Float%20%28double-precision%29) (TriggeredSeconds :type Float%20%28double-precision%29) (InputAction :type Input%20Action%20Object%20Reference :default "/Game/MyContent/Player/Inputs/IA_TurnCamera.IA_TurnCamera"))
  (Class|MGCharacter|PureRotateCharacter (Variables|Default|GetCharRef) ActionValue))

(event Input|EnhancedActionEvents|EnhancedInputActionIA_Shoot
  (params (ActionValue :type Boolean) (ElapsedSeconds :type Float%20%28double-precision%29) (TriggeredSeconds :type Float%20%28double-precision%29) (InputAction :type Input%20Action%20Object%20Reference :default "/Game/MyContent/Player/Inputs/IA_Shoot.IA_Shoot"))
  (Default|PullWeaponTrigger (Variables|Default|GetCharRef) ActionValue))

(event Input|EnhancedActionEvents|EnhancedInputActionIA_Aim
  (params (ActionValue :type Boolean) (ElapsedSeconds :type Float%20%28double-precision%29) (TriggeredSeconds :type Float%20%28double-precision%29) (InputAction :type Input%20Action%20Object%20Reference :default "/Game/MyContent/Player/Inputs/IA_Aim.IA_Aim"))
  (Default|AimDownSights (Variables|Default|GetCharRef) ActionValue))

(event Input|EnhancedActionEvents|EnhancedInputActionIA_Info
  (params (ActionValue :type Boolean) (ElapsedSeconds :type Float%20%28double-precision%29) (TriggeredSeconds :type Float%20%28double-precision%29) (InputAction :type Input%20Action%20Object%20Reference :default "/Game/MyContent/Player/Inputs/IA_Info.IA_Info"))
  (bind _scoreboard (Variables|Default|GetScoreBoard))
  (if ActionValue
    (Widget|SetVisibility _scoreboard "Visible")
    (Default|Refresh _scoreboard)
    (else
      (Widget|SetVisibility (Variables|Default|GetScoreBoard) "Collapsed"))))

(event Input|EnhancedActionEvents|EnhancedInputActionIA_Dash
  (params (ActionValue :type Boolean) (ElapsedSeconds :type Float%20%28double-precision%29) (TriggeredSeconds :type Float%20%28double-precision%29) (InputAction :type Input%20Action%20Object%20Reference :default "/Game/MyContent/Player/Inputs/IA_Dash.IA_Dash"))
  (Class|MGCharacter|TryDash (Variables|Default|GetCharRef) (stale Input|EnhancedActionEvents|EnhancedInputActionIA_Move ActionValue)))

(event Input|EnhancedActionEvents|EnhancedInputActionIA_SpecialReload
  (params (ActionValue :type Boolean) (ElapsedSeconds :type Float%20%28double-precision%29) (TriggeredSeconds :type Float%20%28double-precision%29) (InputAction :type Input%20Action%20Object%20Reference :default "/Game/MyContent/Player/Inputs/IA_SpecialReload.IA_SpecialReload"))
  (bind _charref (Variables|Default|GetCharRef))
  (if (Variables|/Game/MyContent/Characters/BP_Character.BP_Character_C|GetCan%20Critical%20Reload? _charref)
    (Default|LocalAddAmmo _charref true)
    (else
      (Default|SetLockoutLocal _charref))))

(event Input|EnhancedActionEvents|EnhancedInputActionIA_SpecialShoot
  (params (ActionValue :type Boolean) (ElapsedSeconds :type Float%20%28double-precision%29) (TriggeredSeconds :type Float%20%28double-precision%29) (InputAction :type Input%20Action%20Object%20Reference :default "/Game/MyContent/Player/Inputs/IA_SpecialShoot.IA_SpecialShoot")))

(event Input|EnhancedActionEvents|EnhancedInputActionIA_Reload
  (params (ActionValue :type Boolean) (ElapsedSeconds :type Float%20%28double-precision%29) (TriggeredSeconds :type Float%20%28double-precision%29) (InputAction :type Input%20Action%20Object%20Reference :default "/Game/MyContent/Player/Inputs/IA_Reload.IA_Reload"))
  (Default|TryReload (Variables|Default|GetCharRef)))

(event EventPureonRepPosess
  (params (PossessedPawn :type Pawn%20Object%20Reference))
  (if (Pawn|IsLocalPlayerController)
    (Utilities|FlowControl|DoOnce false
      (:Completed
        (bind _asbp_character (Utilities|Casting|CastToBP_Character PossessedPawn))
        (Variables|Default|SetCharRef _asbp_character)
        (Input|AddMappingContext (PlayerController|LocalPlayerSubsystems|GetEnhancedInputLocalPlayerSubsystem) "/Game/MyContent/Player/Inputs/IMC_CharacterControls.IMC_CharacterControls" 0 "(bIgnoreAllPressedKeysUntilRelease=True,bForceImmediately=False,bNotifyUserSettings=False)")
        (CallFunction|AddAttackIMC)
        (bind _returnvalue (UserInterface|CreateWidget "/Game/MyContent/UI/BP_UI_PlayerHud.BP_UI_PlayerHud_C" self))
        (bind _output_get (Variables|Default|SetPlayer%20Hud _returnvalue))
        (UserInterface|Viewport|AddtoPlayerScreen _output_get)
        (bind _returnvalue_2 (UserInterface|CreateWidget "/Game/MyContent/UI/UW_ScoreBoard.UW_ScoreBoard_C" self))
        (bind _output_get_2 (Variables|Default|SetScoreBoard _returnvalue_2))
        (UserInterface|Viewport|AddtoPlayerScreen _output_get_2)
        (Widget|SetVisibility (Variables|Default|GetScoreBoard) "Collapsed")
        (bind _returnvalue_3 (UserInterface|CreateWidget "/Game/MyContent/UI/UI_Reload.UI_Reload_C" self))
        (bind _output_get_3 (Variables|Default|SetReload _returnvalue_3))
        (UserInterface|Viewport|AddtoPlayerScreen _output_get_3)
        (Widget|SetVisibility (Variables|Default|GetReload) "Collapsed")))))

(fn ConstructionScript)

(fn ReloadAnim
  (params (Critical%20Spot :type Float%20%28double-precision%29) (Play%20time :type Float%20%28double-precision%29))
  (Widget|SetVisibility (Variables|Default|GetReload) "Visible")
  (Default|PlayBarAnim (Variables|Default|GetReload) Critical%20Spot Play%20time))

(fn RemoveAttackIMC
  (Input|RemoveMappingContext (PlayerController|LocalPlayerSubsystems|GetEnhancedInputLocalPlayerSubsystem) "/Game/MyContent/Player/Inputs/IMC_Attacks.IMC_Attacks" "(bIgnoreAllPressedKeysUntilRelease=True,bForceImmediately=False,bNotifyUserSettings=False)")
  (Input|AddMappingContext (PlayerController|LocalPlayerSubsystems|GetEnhancedInputLocalPlayerSubsystem) "/Game/MyContent/Player/Inputs/IMC_Reload.IMC_Reload" 0 "(bIgnoreAllPressedKeysUntilRelease=True,bForceImmediately=False,bNotifyUserSettings=False)"))

(fn AddAttackIMC
  (Input|AddMappingContext (PlayerController|LocalPlayerSubsystems|GetEnhancedInputLocalPlayerSubsystem) "/Game/MyContent/Player/Inputs/IMC_Attacks.IMC_Attacks" 0 "(bIgnoreAllPressedKeysUntilRelease=True,bForceImmediately=False,bNotifyUserSettings=False)")
  (Input|RemoveMappingContext (PlayerController|LocalPlayerSubsystems|GetEnhancedInputLocalPlayerSubsystem) "/Game/MyContent/Player/Inputs/IMC_Reload.IMC_Reload" "(bIgnoreAllPressedKeysUntilRelease=True,bForceImmediately=False,bNotifyUserSettings=False)"))

(fn RemoveReload
  (Widget|SetVisibility (Variables|Default|GetReload) "Collapsed"))

(fn UpdateAmmoCount
  (params (Ammo :type Integer))
  (Default|UpdateAmmo (Variables|Default|GetPlayer%20Hud) Ammo))