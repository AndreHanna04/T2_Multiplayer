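; BP_MyPlayerState is a player state that tracks one player's kill and death counts.
; AddKill and AddDeath increment their counter and immediately call the matching KillCountChanged or DeathCountChanged notification.
; Each counter's OnRep function calls the same notification, so replicated updates announce changes too.
; The event graph and construction script hold no logic.
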(event EventBeginPlay)

(event EventTick
  (params (DeltaSeconds :type Float%20%28single-precision%29)))

(fn ConstructionScript)

(fn OnRepKillCount
  (Default|CallKillCountChanged))

(fn AddKill
  (Math|Integer|IncrementInt (Variables|Default|GetKillCount)
    (:%20%20
      (Default|CallKillCountChanged))))

(fn AddDeath
  (Math|Integer|IncrementInt (Variables|Default|GetDeathCount)
    (:%20%20
      (Default|CallDeathCountChanged))))

(fn OnRepDeathCount
  (Default|CallDeathCountChanged))