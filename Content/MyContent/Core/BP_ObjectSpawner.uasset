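; BP_ObjectSpawner scatters randomly rotated BP_Object actors around itself within the radius of its Sphere component.
; RefreshObjects destroys BP_Object actors found within twice that radius, then spawns NumberOfObjects new ones in the outer half of the radius, calling SetObject on each.
; ClearObjects performs only the overlap-based removal.
; Cleanup relies on the overlap query rather than stored references, and nothing here runs automatically.
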(event EventBeginPlay)

(event Collision|EventActorBeginOverlap
  (params (OtherActor :type Actor%20Object%20Reference)))

(event EventTick
  (params (DeltaSeconds :type Float%20%28single-precision%29)))

(fn ConstructionScript)

(fn RefreshObjects
  (bind _outactors (Collision|SphereOverlapActors (Transformation|GetActorLocation) (* (Components|Sphere|GetScaledSphereRadius (Variables|Default|GetSphere)) 2.0) (LocalVariables|GetNewLocalVar) "/Game/MyContent/Core/BP_Object.BP_Object_C"))
  (for _array_element _outactors
    (Actor|DestroyActor _array_element))
  (for _index (range 1 (Variables|Default|GetNumber%20Of%20Objects))
    (bind _returnvalue (Game|SpawnActorfromClass "/Game/MyContent/Core/BP_Object.BP_Object_C" (Math|Transform|MakeTransform (+ (* (Math|Random|RandomUnitVector) (* (Components|Sphere|GetScaledSphereRadius (Variables|Default|GetSphere)) (Math|Random|RandomFloatinRange 0.5 1.0))) (Transformation|GetActorLocation)) (Math|Random|RandomRotator false) "1.000000,1.000000,1.000000") "Undefined" "MultiplyWithRoot" 0 0))
    (Default|SetObject _returnvalue)))

(fn ClearObjects
  (bind _outactors (Collision|SphereOverlapActors (Transformation|GetActorLocation) (* (Components|Sphere|GetScaledSphereRadius (Variables|Default|GetSphere)) 2.0) (LocalVariables|GetNewLocalVar_0) "/Game/MyContent/Core/BP_Object.BP_Object_C"))
  (for _array_element _outactors
    (Actor|DestroyActor _array_element)))