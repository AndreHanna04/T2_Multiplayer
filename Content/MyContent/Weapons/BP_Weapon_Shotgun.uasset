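; BP_Weapon_Shotgun is a shotgun weapon that fires a spread of line-damage traces along the shot direction.
; Its Activate Damage function loops over pellets, each taking a random direction in a cone that widens with the loop index, scaled by Range.
; Traces start slightly ahead of the shot location with timed debug drawing enabled.
; Back force is applied once per pellet, so it repeats within a single shot.
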(event EventBeginPlay
  (|CallParentFunction) ; This node is disabled and will not be called.\nDrag off pins to build functionality.
)

(event Collision|EventActorBeginOverlap
  (params (OtherActor :type Actor%20Object%20Reference))
  (|CallParentFunction OtherActor) ; This node is disabled and will not be called.\nDrag off pins to build functionality.
)

(event EventTick
  (params (DeltaSeconds :type Float%20%28single-precision%29))
  (|CallParentFunction DeltaSeconds) ; This node is disabled and will not be called.\nDrag off pins to build functionality.
)

(fn ConstructionScript
  (|CallParentFunction))

(fn ActivateDamage
  (params (Shoot%20Loc :type Vector :default "0, 0, 0") (Shoot%20Dir :type Vector :default "0, 0, 0"))
  (for _index (range 0 10)
    (CallFunction|ApplyLineDamage (+ Shoot%20Loc (* Shoot%20Dir 3.0)) (* (Math|Random|RandomUnitVectorinConeinDegrees Shoot%20Dir (* _index 0.8)) (Variables|Default|GetRange)) "ForDuration")
    (CallFunction|ApplyBackForce)))